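; PC_Mouse is a player controller that drives mouse and touch input for a two-player chess game.
; On left-click or touch release it passes the location hit under the cursor and the current player to BP_ChessBoard's Click, storing the result as the active player.
; When the board's LastClick is -1 and Move is set, it plays a level sequence transitioning between the two players' sides, chosen by whose turn it is.
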(event `self.ReceiveBeginPlay`
  (set `self.bShowMouseCursor` true))

(event `Key|LeftMouseButton`
  (params (Key :type "Key Structure" :default "AnyKey"))
  (bind _chessboardclass (`self.ChessBoardClass`))
  (:`Released`
    (bind _outactors (`GameplayStatics.GetAllActorsOfClass` "/Game/BluePrints/BP_ChessBoard.BP_ChessBoard_C" :!label _label))
    (set `self.ChessBoardClass` (`KismetArrayLibrary.Array_Get` _outactors))
    (bind _player1 (`/Game/BluePrints/BP_ChessBoard.Click` (`self.ChessBoardClass`) (`.Location` (`GameplayStatics.BreakHitResult` (`self.GetHitResultUnderCursorByChannel` "TraceTypeQuery1"))) (`self.Player1`)))
    (set `self.Player1` _player1)
    (if (and (== (`/Game/BluePrints/BP_ChessBoard.LastClick` _chessboardclass) -1) (`/Game/BluePrints/BP_ChessBoard.Move` _chessboardclass))
      (if _player1
        (`/Engine/EditorBlueprintResources/StandardMacros.DoOnce` false :!label _label_2
          (:`Completed`
            (bind _returnvalue (`LevelSequencePlayer.CreateLevelSequencePlayer` "/Game/BluePrints/Player2ToPlayer1.Player2ToPlayer1"))
            (`MovieSceneSequencePlayer.Play` _returnvalue)
            (goto _label_2 :!via `Reset`)))
        (else
          (`/Engine/EditorBlueprintResources/StandardMacros.DoOnce` false :!label _label_3
            (:`Completed`
              (bind _returnvalue_2 (`LevelSequencePlayer.CreateLevelSequencePlayer` "/Game/BluePrints/Player1ToPlayer2.Player1ToPlayer2"))
              (`MovieSceneSequencePlayer.Play` _returnvalue_2)
              (goto _label_3 :!via `Reset`))))))))

(event `InputTouch`
  (params (Location :type "Vector Structure") (FingerIndex :type "ETouchIndex Enum"))
  (:`Released`
    (goto _label)))

(fn `UserConstructionScript`)