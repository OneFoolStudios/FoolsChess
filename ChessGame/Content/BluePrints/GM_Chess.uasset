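; Game mode for a chess game that manages the main menu, match reset and win screens.
; BeginPlay opens the menu and caches PC_Mouse; ResetGame gives Player1 the turn, respawns BP_ChessBoard and shows WhitePlayerHUD.
; EndGame adds the black or white win widget based on the board's BlackWin flag.
; PutTheFiguresBackInPlace, not called here, restores the board's start arrays and rebuilds piece meshes from tile indices.
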(event `self.ReceiveBeginPlay`
  (`self.CreateMainMenu`)
  (bind _outactors (`GameplayStatics.GetAllActorsOfClass` "/Game/Blueprints/PC_Mouse.PC_Mouse_C"))
  (set `self.MouseClass` (`KismetArrayLibrary.Array_Get` _outactors)))

(event `self.ReceiveTick`
  (params (DeltaSeconds :type "Float (single-precision)")))

(event `CreateMainMenu`
  (`WidgetLayoutLibrary.RemoveAllWidgets`)
  (bind _returnvalue (`|CreateWidget` "/Game/BluePrints/MainMenu.MainMenu_C" (`GameplayStatics.GetPlayerController` 0)))
  (`UserWidget.AddToViewport` _returnvalue 0))

(event `ResetGame`
  (set `/Game/Blueprints/PC_Mouse.Player1` true (`self.MouseClass`))
  (`self.K2_DestroyActor` (`self.ChessBoardClass`))
  (bind _returnvalue (`|SpawnActorFromClass` "/Game/BluePrints/BP_ChessBoard.BP_ChessBoard_C" (`KismetMathLibrary.MakeTransform` (0.0 0.0 0.0)) "Undefined" "OverrideRootScale"))
  (set `self.ChessBoardClass` _returnvalue)
  (`self.CreatePlayerHUD`))

(event `EndGame`
  (bind _returnvalue (`GameplayStatics.GetPlayerController` 0))
  (if (`/Game/BluePrints/BP_ChessBoard.BlackWin` (`self.ChessBoardClass`))
    (bind _returnvalue_2 (`|CreateWidget` "/Game/BluePrints/BlackWins.BlackWins_C" _returnvalue))
    (`UserWidget.AddToViewport` _returnvalue_2 0)
    (else
      (bind _returnvalue_3 (`|CreateWidget` "/Game/BluePrints/WhiteWins.WhiteWins_C" _returnvalue))
      (`UserWidget.AddToViewport` _returnvalue_3 0))))

(event `CreatePlayerHUD`
  (`WidgetLayoutLibrary.RemoveAllWidgets`)
  (bind _aspc_mouse (cast `/Game/Blueprints/PC_Mouse` (`GameplayStatics.GetPlayerController` 0)))
  (bind _returnvalue (`|CreateWidget` "/Game/BluePrints/WhitePlayerHUD.WhitePlayerHUD_C" _aspc_mouse))
  (`UserWidget.AddToViewport` _returnvalue 0))

(fn `PutTheFiguresBackInPlace`
  (bind _chessboardclass (`self.ChessBoardClass`))
  (bind _indextile (`self.IndexTile`))
  (bind _returnvalue (< _indextile 30))
  (bind _startarrayfig (`/Game/BluePrints/BP_ChessBoard.StartArrayFig` _chessboardclass))
  (set `/Game/BluePrints/BP_ChessBoard.UpdatedArrayColor` (`/Game/BluePrints/BP_ChessBoard.StartArrayColor` _chessboardclass) _chessboardclass)
  (set `/Game/BluePrints/BP_ChessBoard.UpdatedArrayFig` _startarrayfig _chessboardclass)
  (for _index (range 64)
    (set `self.IndexTile` _index)
    (bind _returnvalue_2 (`AddComponent|NODE_AddStaticMeshComponent-0` :`RelativeTransform` (`KismetMathLibrary.Conv_VectorToTransform` (`self.IndexToPosition300` _indextile))))
    (`ActorComponent.K2_DestroyComponent` (`KismetArrayLibrary.Array_Get` (`/Game/BluePrints/BP_ChessBoard.PiecesMesh` _chessboardclass) _indextile))
    (`StaticMeshComponent.SetStaticMesh` _returnvalue_2 (select `int` (`KismetArrayLibrary.Array_Get` _startarrayfig _indextile) :`0` null :`1` "/Game/Props/SM_Pion.SM_Pion" :`2` "/Game/Props/SM_Tower.SM_Tower" :`3` "/Game/Props/SM_Horse.SM_Horse" :`4` "/Game/Props/SM_Loperl.SM_Loperl" :`5` "/Game/Props/SM_Queen.SM_Queen" :`6` "/Game/Props/SM_King.SM_King" :!type "StaticMesh Object Reference"))
    (`PrimitiveComponent.SetMaterial` _returnvalue_2 0 (select `bool` _returnvalue :`false` "/Game/Props/Black_Piece.Black_Piece" :`true` "/Game/Props/White_piece.White_piece" :!type "Material Object Reference"))
    (`KismetArrayLibrary.Array_Add` (`/Game/BluePrints/BP_ChessBoard.PiecesMesh` (`self.ChessBoardClass`)) _returnvalue_2)
    (if _returnvalue
      (`SceneComponent.K2_AddRelativeRotation` _returnvalue_2 (struct :`Yaw` 180.0) false false))))

(fn `UserConstructionScript`)