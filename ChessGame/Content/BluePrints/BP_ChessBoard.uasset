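; Chess board actor that builds the squares and pieces in its construction script and runs a two-player game.
; Click selects and highlights a piece, then dispatches the second click to per-piece move rules with blocking and capture checks.
; Valid moves update flat 64-index figure and color arrays, respawn the mesh and swap the turn HUD.
; Captures compare piece materials to tell sides apart, and attacking a king ends the game through GM_Chess.
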(fn `Click`
  (params (Position :type "Vector Structure") (WhitePlayer :type Boolean))
  (returns (Player1 :type Boolean))
  (bind _returnvalue (`self.PositionToIndex` Position))
  (bind _lastclick (`self.LastClick`))
  (bind _player1 (`self.Player1`))
  (bind _returnvalue_2 (not _player1))
  (bind _returnvalue_3 (== (`self.LastClick`) -1))
  (set `self.Player1` WhitePlayer)
  (set `self.Move` false)
  (set `self.ActiveClick` _returnvalue)
  (if (and (== (`KismetArrayLibrary.Array_Get` (`self.UpdatedArrayColor`) _returnvalue) (select `bool` WhitePlayer :`false` 2 :`true` 1)) _returnvalue_3)
    _
    (elif (!= _returnvalue_3 true)
      _
      (else
        (return (`self.Player1`)))))
  (if (== (`self.LastClick`) -1)
    ;[1 1 1] The First Click
    ;;[1 1 1] Light up selected Tile
    (`PrimitiveComponent.SetMaterial` (`KismetArrayLibrary.Array_Get` (`self.TileFieldMesh`) (`self.ActiveClick`)) 0 "/Game/Props/M_Border.M_Border")
    (set `self.LastClick` (`self.ActiveClick`))
    (else
      ;[1 1 1] Color The selected tile back to the origin color
      (`PrimitiveComponent.SetMaterial` (`KismetArrayLibrary.Array_Get` (`self.TileFieldMesh`) _lastclick) 0 (`KismetArrayLibrary.Array_Get` (`self.TileFieldMat`) _lastclick))
      (bind (_dy _dx _biggest _lowest) (`self.DiffXAndY` _lastclick (`self.ActiveClick`)))
      (set `self.DifferenceY` _dy)
      (set `self.DifferenceX` _dx)
      (set `self.BiggestCo` _biggest)
      (set `self.LowestCo` _lowest)
      (switch `int` (`KismetArrayLibrary.Array_Get` (`self.UpdatedArrayFig`) _lastclick)
        (:`Default`
          _)
        (:`0`
          _)
        (:`1`
          (`self.PionLogic`)
          (if (or (`self.WhiteWin`) (`self.BlackWin`)) :!label _label
            (`/Game/BluePrints/GM_Chess.EndGame` (cast `/Game/BluePrints/GM_Chess` (`GameplayStatics.GetGameMode`) :!pure true))
            (bind _output_get (set `self.Player1` true))
            (return _output_get)
            (elif (`self.Move`)
              (if _returnvalue_2
                (`WidgetLayoutLibrary.RemoveAllWidgets`)
                (bind _returnvalue_4 (`|CreateWidget` "/Game/BluePrints/WhitePlayerHUD.WhitePlayerHUD_C"))
                (`UserWidget.AddToViewport` _returnvalue_4 0)
                (else
                  (`WidgetLayoutLibrary.RemoveAllWidgets`)
                  (bind _returnvalue_5 (`|CreateWidget` "/Game/BluePrints/BlackPlayerHUD.BlackPlayerHUD_C"))
                  (`UserWidget.AddToViewport` _returnvalue_5 0)))
              (return _returnvalue_2)
              (else
                (return _player1)))))
        (:`2`
          (`self.TowerLogic`)
          (goto _label))
        (:`3`
          (`self.HorseLogic`)
          (goto _label))
        (:`4`
          (`self.LoperLogic`)
          (goto _label))
        (:`5`
          (`self.QueenLogic`)
          (goto _label))
        (:`6`
          (`self.KingLogic`)
          (goto _label)))
      (set `self.LastClick` -1)))
  (return (`self.Player1`)))

(fn `DiffXAndY`
  (params (LastIndex :type Integer) (ActiveIndex :type Integer))
  (returns (dY :type Integer) (dX :type Integer) (Biggest :type "Vector2D Structure") (Lowest :type "Vector2D Structure"))
  (locals (DiffX :type Integer) (DiffY :type Integer) (BigX :type "Float (double-precision)" :default 0.0) (lowX :type "Float (double-precision)" :default 0.0) (BigY :type "Float (double-precision)" :default 0.0) (LowY :type "Float (double-precision)" :default 0.0))
  (bind (_x _y) (`self.IndexToSimpleCo` LastIndex))
  (bind (_x_2 _y_2) (`self.IndexToSimpleCo` ActiveIndex))
  (bind _returnvalue (`KismetMathLibrary.Conv_IntToDouble` _x))
  (bind _returnvalue_2 (`KismetMathLibrary.Conv_IntToDouble` _x_2))
  (bind _returnvalue_3 (`KismetMathLibrary.Conv_IntToDouble` _y_2))
  (bind _returnvalue_4 (`KismetMathLibrary.Conv_IntToDouble` _y))
  (bind _returnvalue_5 (- _x_2 _x))
  (bind _returnvalue_6 (- _y _y_2))
  (if (>= _x _x_2)
    (set `local.BigX` _returnvalue)
    (set `local.lowX` _returnvalue_2)
    (else
      (set `local.BigX` _returnvalue_2)
      (set `local.lowX` _returnvalue)))
  (if (>= _y_2 _y)
    (set `local.BigY` _returnvalue_3)
    (set `local.LowY` _returnvalue_4)
    (else
      (set `local.BigY` _returnvalue_4)
      (set `local.LowY` _returnvalue_3)))
  (if (> _returnvalue_5 0)
    (set `local.DiffX` _returnvalue_5)
    (else
      (set `local.DiffX` (* _returnvalue_5 -1))))
  (if (> _returnvalue_6 0)
    (set `local.DiffY` _returnvalue_6)
    (else
      (set `local.DiffY` (* _returnvalue_6 -1))))
  (return (`local.DiffY`) (`local.DiffX`) (`KismetMathLibrary.MakeVector2D` (`local.BigX`) (`local.BigY`)) (`KismetMathLibrary.MakeVector2D` (`local.lowX`) (`local.LowY`))))

(fn `HorseLogic`
  (bind _differencex (`self.DifferenceX`))
  (bind _differencey (`self.DifferenceY`))
  (if (and (== _differencex 2) (== _differencey 1))
    (if (== (`self.CheckWhatPieceOnActiveLocation`) 0) :!label _label
      (`self.MoveAndUpdatePiece` :!label _label_2)
      (return)
      (else
        (`self.CheckIfTargetLocationIsDifferentColor`
          (:`then`
            (goto _label_2))
          (:`else`
            _))))
    (elif (and (== _differencex 1) (== _differencey 2))
      (goto _label)
      (else
        _)))
  (set `self.LastClick` -1))

(fn `KingLogic`
  (bind _differencey (`self.DifferenceY`))
  (bind _differencex (`self.DifferenceX`))
  (if (and (or (== _differencex 0) (== _differencex 1)) (or (== _differencey 0) (== _differencey 1)))
    (if (== (`self.CheckWhatPieceOnActiveLocation`) 0)
      (`self.MoveAndUpdatePiece` :!label _label)
      (return)
      (else
        (`self.CheckIfTargetLocationIsDifferentColor`
          (:`then`
            (goto _label))
          (:`else`
            (set `self.LastClick` -1)))))
    (else
      (set `self.LastClick` -1))))

(fn `LoperLogic`
  (bind _differencex (`self.DifferenceX`))
  (if (== _differencex (`self.DifferenceY`))
    (if (<= (`.Y` (`self.IndexToSimpleCo` (`self.LastClick`))) (`.Y` (`self.IndexToSimpleCo` (`self.ActiveClick`))))
      (set `self.LoperLeftOrRight` 1)
      (else
        (set `self.LoperLeftOrRight` -1)))
    (for _index (range 1 _differencex)
      (bind _output_get (set `self.NothingInTheWay` (!= (`KismetArrayLibrary.Array_Get` (`self.UpdatedArrayFig`) (+ (* _index 8) (* _index (`self.LoperLeftOrRight`)) (`self.LastClick`))) 0)))
      (if _output_get
        (break)))
    (if (`self.NothingInTheWay`)
      _
      (elif (== (`self.CheckWhatPieceOnActiveLocation`) 0)
        (`self.MoveAndUpdatePiece` :!label _label)
        (return)
        (else
          (`self.CheckIfTargetLocationIsDifferentColor`
            (:`then`
              (goto _label))
            (:`else`
              _)))))
    (set `self.NothingInTheWay` false))
  (set `self.LastClick` -1))

(fn `MoveAndUpdatePiece`
  (bind _lastclick (`self.LastClick`))
  (bind _activeclick (`self.ActiveClick`))
  (`self.UpdateFigureArray` (`KismetArrayLibrary.Array_Get` (`self.UpdatedArrayFig`) _lastclick))
  (`ActorComponent.K2_DestroyComponent` (`KismetArrayLibrary.Array_Get` (`self.PiecesMesh`) _lastclick))
  (bind _returnvalue (`AddComponent|NODE_AddStaticMeshComponent-11` :`RelativeTransform` (`KismetMathLibrary.Conv_VectorToTransform` (`self.IndexToPosition300` _activeclick))))
  (`StaticMeshComponent.SetStaticMesh` _returnvalue (`KismetArrayLibrary.Array_Get` (`self.ArrayFig`) (`KismetArrayLibrary.Array_Get` (`self.UpdatedArrayFig`) _activeclick)))
  (`KismetArrayLibrary.Array_Set` (`self.PiecesMesh`) _activeclick _returnvalue)
  (`PrimitiveComponent.SetMaterial` _returnvalue 0 (select `bool` (== (`KismetArrayLibrary.Array_Get` (`self.UpdatedArrayColor`) (`self.LastClick`)) 1) :`false` "/Game/Props/Black_Piece.Black_Piece" :`true` "/Game/Props/White_piece.White_piece" :!type "Material Object Reference"))
  (`self.UpdateColorArray`)
  (set `self.LastClick` -1)
  (set `self.Move` true)
  (return))

(fn `PionLogic`
  (bind _item (`self.CheckWhatPieceOnActiveLocation`))
  (bind (_x _y) (`self.IndexToSimpleCo` (`self.LastClick`)))
  (bind (_x_2 _y_2) (`self.IndexToSimpleCo` (`self.ActiveClick`)))
  (bind _returnvalue (- _y _y_2))
  (bind _returnvalue_2 (== _returnvalue 0))
  (bind _returnvalue_3 (* (select `bool` (`self.Player1`) :`false` -1 :`true` 1) (- _x_2 _x)))
  (bind _returnvalue_4 (== _returnvalue_3 1))
  (if (and (and _returnvalue_4 _returnvalue_2) (== _item 0))
    (`self.MoveAndUpdatePiece` :!label _label)
    (return)
    (else
      (if (and (or (and _returnvalue_4 (== _returnvalue 1)) (and _returnvalue_4 (== _returnvalue -1))) (!= _item 0))
        (`self.CheckIfTargetLocationIsDifferentColor`
          (:`then`
            (goto _label))
          (:`else`
            _))
        (elif (and (and (== _returnvalue_3 2) _returnvalue_2) (== (`KismetArrayLibrary.Array_Get` (`self.StartArrayFig`) (`self.LastClick`)) 1))
          (goto _label)
          (else
            _)))
      (set `self.LastClick` -1))))

(fn `QueenLogic`
  (bind _differencex (`self.DifferenceX`))
  (bind (_biggestco_x _biggestco_y) (`KismetMathLibrary.BreakVector2D` (`self.BiggestCo`)))
  (bind (_lowestco_x _lowestco_y) (`KismetMathLibrary.BreakVector2D` (`self.LowestCo`)))
  (bind _returnvalue (== (`self.DifferenceX`) 0))
  (bind _returnvalue_2 (== (`self.DifferenceY`) 0))
  (bind _returnvalue_3 (`KismetMathLibrary.FTrunc` _lowestco_y))
  (bind _returnvalue_4 (`KismetMathLibrary.FTrunc` _biggestco_x))
  (if (xor _returnvalue _returnvalue_2)
    ;[1 1 1] Check if somthing is in the way?
    ;;[1 1 1] X=0
    (if _returnvalue
      (for _index (range (+ _returnvalue_3 1) (`KismetMathLibrary.FTrunc` _biggestco_y))
        (bind _output_get (set `self.NothingInTheWay` (!= (`KismetArrayLibrary.Array_Get` (`self.UpdatedArrayFig`) (+ _index (* _returnvalue_4 8))) 0)))
        (if _output_get
          (break)))
      (if (`self.NothingInTheWay`)
        (set `self.LastClick` -1 :!label _label)
        (set `self.NothingInTheWay` false)
        (else
          (if (== (`self.CheckWhatPieceOnActiveLocation`) 0) :!label _label_2
            (`self.MoveAndUpdatePiece` :!label _label_3)
            (return)
            (else
              (`self.CheckIfTargetLocationIsDifferentColor`
                (:`then`
                  (goto _label_3))
                (:`else`
                  (set `self.LastClick` -1)))))))
      (else
        ;;[1 1 1] Y=0
        (if _returnvalue_2
          (for _index_2 (range (+ (`KismetMathLibrary.FTrunc` _lowestco_x) 1) _returnvalue_4)
            (bind _output_get_2 (set `self.NothingInTheWay` (!= (`KismetArrayLibrary.Array_Get` (`self.UpdatedArrayFig`) (+ (* _index_2 8) _returnvalue_3)) 0)))
            (if _output_get_2
              (break)))
          (if (`self.NothingInTheWay`)
            (goto _label)
            (else
              (goto _label_2))))))
    (elif (== _differencex (`self.DifferenceY`))
      (if (<= (`.Y` (`self.IndexToSimpleCo` (`self.LastClick`))) (`.Y` (`self.IndexToSimpleCo` (`self.ActiveClick`))))
        (set `self.LoperLeftOrRight` 1)
        (else
          (set `self.LoperLeftOrRight` -1)))
      (for _index_3 (range 1 _differencex)
        (bind _output_get_3 (set `self.NothingInTheWay` (!= (`KismetArrayLibrary.Array_Get` (`self.UpdatedArrayFig`) (+ (* _index_3 8) (* _index_3 (`self.LoperLeftOrRight`)) (`self.LastClick`))) 0)))
        (if _output_get_3
          (break)))
      (if (`self.NothingInTheWay`)
        _
        (elif (== (`self.CheckWhatPieceOnActiveLocation`) 0)
          (`self.MoveAndUpdatePiece` :!label _label_4)
          (return)
          (else
            (`self.CheckIfTargetLocationIsDifferentColor`
              (:`then`
                (goto _label_4))
              (:`else`
                _)))))
      (set `self.LastClick` -1)
      (set `self.NothingInTheWay` false)
      (else
        (set `self.LastClick` -1)))))

(fn `TowerLogic`
  (bind (_biggestco_x _biggestco_y) (`KismetMathLibrary.BreakVector2D` (`self.BiggestCo`)))
  (bind (_lowestco_x _lowestco_y) (`KismetMathLibrary.BreakVector2D` (`self.LowestCo`)))
  (bind _returnvalue (== (`self.DifferenceX`) 0))
  (bind _returnvalue_2 (== (`self.DifferenceY`) 0))
  (bind _returnvalue_3 (`KismetMathLibrary.FTrunc` _lowestco_y))
  (bind _returnvalue_4 (`KismetMathLibrary.FTrunc` _biggestco_x))
  (if (xor _returnvalue _returnvalue_2)
    ;[1 1 1] Check if somthing is in the way?
    ;;[1 1 1] X=0
    (if _returnvalue
      (for _index (range (+ _returnvalue_3 1) (`KismetMathLibrary.FTrunc` _biggestco_y))
        (bind _output_get (set `self.NothingInTheWay` (!= (`KismetArrayLibrary.Array_Get` (`self.UpdatedArrayFig`) (+ _index (* _returnvalue_4 8))) 0)))
        (if _output_get
          (break)))
      (if (`self.NothingInTheWay`)
        (set `self.NothingInTheWay` false :!label _label)
        (else
          (if (== (`self.CheckWhatPieceOnActiveLocation`) 0) :!label _label_2
            (`self.MoveAndUpdatePiece` :!label _label_3)
            (return)
            (else
              (`self.CheckIfTargetLocationIsDifferentColor`
                (:`then`
                  (goto _label_3))
                (:`else`
                  _))))))
      (else
        ;;[1 1 1] Y=0
        (if _returnvalue_2
          (for _index_2 (range (+ (`KismetMathLibrary.FTrunc` _lowestco_x) 1) _returnvalue_4)
            (bind _output_get_2 (set `self.NothingInTheWay` (!= (`KismetArrayLibrary.Array_Get` (`self.UpdatedArrayFig`) (+ (* _index_2 8) _returnvalue_3)) 0)))
            (if _output_get_2
              (break)))
          (if (`self.NothingInTheWay`)
            (goto _label)
            (else
              (goto _label_2)))
          (else
            _)))))
  (set `self.LastClick` -1))

(fn `UserConstructionScript`
  (bind _indextile (`self.IndexTile`))
  (bind _indextile_2 (`self.IndexTile`))
  (bind _returnvalue (< _indextile 30))
  (bind _returnvalue_2 (select `bool` (xor (`KismetMathLibrary.Conv_IntToBool` (mod _indextile_2 2)) (`KismetMathLibrary.Conv_IntToBool` (mod (/ _indextile_2 8) 2))) :`false` "/Game/Props/Black_Square.Black_Square" :`true` "/Game/Props/White_Square.White_Square" :!type "Material Object Reference"))
  ;[1 1 1] SchaakBord aanmaken
  (for _index (range 64)
    (set `self.IndexTile` _index)
    (`|ExecutionSequence`
      (:`then_0`
        (bind _returnvalue_3 (`AddComponent|NODE_AddStaticMeshComponent-1` :`RelativeTransform` (`KismetMathLibrary.Conv_VectorToTransform` (`self.IndexToPosition` _indextile_2))))
        (`KismetArrayLibrary.Array_Add` (`self.TileFieldMesh`) _returnvalue_3)
        (`PrimitiveComponent.SetMaterial` _returnvalue_3 0 _returnvalue_2)
        (`KismetArrayLibrary.Array_Add` (`self.TileFieldMat`) _returnvalue_2))
      (:`then_1`
        ;[1 1 1] Plaatsen van de peetjes
        (bind _returnvalue_4 (`AddComponent|NODE_AddStaticMeshComponent-8` :`RelativeTransform` (`KismetMathLibrary.Conv_VectorToTransform` (`self.IndexToPosition300` (`self.IndexTile`)))))
        (`StaticMeshComponent.SetStaticMesh` _returnvalue_4 (select `int` (`KismetArrayLibrary.Array_Get` (`self.StartArrayFig`) _indextile) :`0` null :`1` "/Game/Props/SM_Pion.SM_Pion" :`2` "/Game/Props/SM_Tower.SM_Tower" :`3` "/Game/Props/SM_Horse.SM_Horse" :`4` "/Game/Props/SM_Loperl.SM_Loperl" :`5` "/Game/Props/SM_Queen.SM_Queen" :`6` "/Game/Props/SM_King.SM_King" :!type "StaticMesh Object Reference"))
        (`PrimitiveComponent.SetMaterial` _returnvalue_4 0 (select `bool` _returnvalue :`false` "/Game/Props/Black_Piece.Black_Piece" :`true` "/Game/Props/White_piece.White_piece" :!type "Material Object Reference"))
        (`KismetArrayLibrary.Array_Add` (`self.PiecesMesh`) _returnvalue_4)
        ;;[1 1 1] Paarjes draaien
        (if _returnvalue
          (`SceneComponent.K2_AddRelativeRotation` _returnvalue_4 (struct :`Yaw` 180.0) false false))))))